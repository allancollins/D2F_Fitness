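; BP_Player is a player pawn Blueprint with no active gameplay logic in its graphs, as BeginPlay and the construction script are empty.
; The event graph holds only disconnected Asset Registry experiments that never run.
; These include a loop printing the names of all SkeletalMesh assets and unused lookups of the asset count, first asset name and SM_Chicken by object path.
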(event EventBeginPlay)

(fn ConstructionScript)