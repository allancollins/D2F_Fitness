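; Master actor for a display scene: an animated, tintable avatar with a machinery mesh and equipment in each hand.
; The construction script applies meshes and a dynamic material colour; BeginPlay loops animations and snaps equipment to sockets named from hold enums.
; It then blends the view to a chosen or fallback BP_Camera, and a timer steps once through an optional camera list.
; Editor and widget events swap the avatar's mesh and animation.
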(event Custom|UpdateMesh
  (bind _avatarmesh (Variables|Exposed|GetAvatarMesh))
  ;[1 1 1] Editor Logic
  (Utilities|IsValid _avatarmesh
    (:Is%20Valid
      (Class|SkinnedMeshComponent|SetSkeletalMesh (Variables|Components|GetAvatar) _avatarmesh true))))

(event Custom|WidgetUpdateAvatar
  (params (NewMesh :type Skeletal%20Mesh%20Object%20Reference))
  ;[1 1 1] Widget Logic
  (Class|SkinnedMeshComponent|SetSkeletalMesh (Variables|Components|GetAvatar) NewMesh true))

(event Custom|WidgetUpdateAvatarAnimation
  (params (NewAnimToPlay :type Animation%20Asset%20Object%20Reference))
  (bind _avatar (Variables|Components|GetAvatar))
  ;[1 1 1] Widget Logic
  (Components|Animation|SetAnimation _avatar NewAnimToPlay)
  (Components|Animation|PlayAnimation _avatar NewAnimToPlay true))

(event Custom|UpdateAnimation
  (bind _avataranimation (Variables|Exposed|GetAvatarAnimation))
  (bind _avatar (Variables|Components|GetAvatar))
  ;[1 1 1] Editor Logic
  (Utilities|IsValid _avataranimation
    (:Is%20Valid
      (Components|Animation|SetAnimation _avatar _avataranimation)
      (Components|Animation|PlayAnimation _avatar _avataranimation true))))

(event EventBeginPlay
  ;[1 1 1] Begin Play
  (CallFunction|SetAvatarAnimation)
  (CallFunction|SetMachineryAnimation)
  ;;[1 1 1] Hand Socket Names
  (CallFunction|SetHandSocketNames)
  (CallFunction|AttachEquipmenttoHands)
  (CallFunction|SetViewCamera)
  (if (> (Utilities|Array|Length (Variables|Exposed|GetCameraToTransitionTo)) 0)
    (Utilities|Time|SetTimerbyFunctionName 0 "TransitionToCamera" (Variables|Exposed|GetDelayBetweenCameraTransition) true)))

(fn ConstructionScript
  ;[1 1 1] Avatar Setup
  (CallFunction|SetAvatarMesh)
  (CallFunction|CreateAvatarDynamicMaterial)
  (CallFunction|SetAvatarDynamicMaterialColour)
  ;[1 1 1] Machine Mesh
  (CallFunction|SetMachineMesh)
  ;[1 1 1] Equipment Setup
  (CallFunction|SetEquipmentMesh))

(fn SetAvatarMesh
  (Class|SkinnedMeshComponent|SetSkeletalMesh (Variables|Components|GetAvatar) (Variables|Exposed|GetAvatarMesh) true))

(fn SetAvatarAnimation
  (bind _avataranimation (Variables|Exposed|GetAvatarAnimation))
  (Utilities|IsValid _avataranimation
    (:Is%20Valid
      (Components|Animation|PlayAnimation (Variables|Components|GetAvatar) _avataranimation true))))

(fn CreateAvatarDynamicMaterial
  (bind _returnvalue (Rendering|Material|CreateDynamicMaterialInstance (Variables|Components|GetAvatar) 0 0 :!class /Script/Engine.PrimitiveComponent))
  (Variables|Default|SetAvatarMaterials _returnvalue))

(fn SetAvatarDynamicMaterialColour
  (Rendering|Material|SetVectorParameterValue (Variables|Default|GetAvatarMaterials) "Colour Tint" (Math|Conversions|ToLinearColor(Color) (Variables|Exposed|GetColour%20Tint)) :!class /Script/Engine.MaterialInstanceDynamic))

(fn SetMachineMesh
  (Class|SkinnedMeshComponent|SetSkeletalMesh (Variables|Components|GetMachinery) (Variables|Exposed|GetMachineMesh) true))

(fn SetMachineryAnimation
  (bind _machineryanimation (Variables|Exposed|GetMachineryAnimation))
  (Utilities|IsValid _machineryanimation
    (:Is%20Valid
      (Components|Animation|PlayAnimation (Variables|Components|GetMachinery) _machineryanimation true))))

(fn SetHandSocketNames
  (Utilities|FlowControl|Sequence
    (:then_0
      (Variables|Default|SetRightHandSocket (Utilities|String|StringToName (Utilities|String|EnumtoString (Variables|Exposed|GetRightHandEquipmentHold)))))
    (:then_1
      (Variables|Default|SetLeftHandSocket (Utilities|String|StringToName (Utilities|String|EnumtoString (Variables|Exposed|GetLeftHandEquipmentHold)))))))

(fn SetEquipmentMesh
  (bind _leftequipment (Variables|Components|GetLeftEquipment))
  (bind _rightequipment (Variables|Components|GetRightEquipment))
  (Components|StaticMesh|SetStaticMesh _rightequipment (Variables|Exposed|GetRightHandEquipmentMesh))
  (Transformation|SetRelativeLocation _rightequipment (Variables|/Script/Engine.SceneComponent|GetRelativeLocation (Variables|Components|GetRightEquipmentPoint)) false false)
  (Components|StaticMesh|SetStaticMesh _leftequipment (Variables|Exposed|GetLeftHandEquipmentMesh))
  (Transformation|SetRelativeLocation _leftequipment (Variables|/Script/Engine.SceneComponent|GetRelativeLocation (Variables|Components|GetLeftEquipmentPoint)) false false))

(fn AttachEquipmenttoHands
  (Utilities|FlowControl|Sequence
    (:then_0
      (if (!= (Variables|Exposed|GetRightHandEquipmentMesh) 0)
        (Transformation|AttachComponentToComponent (Variables|Components|GetRightEquipment) (Variables|Components|GetAvatar) (Variables|Default|GetRightHandSocket) "SnapToTarget" "KeepRelative" "KeepRelative" true)))
    (:then_1
      (if (!= (Variables|Exposed|GetLeftHandEquipmentMesh) 0)
        (Transformation|AttachComponentToComponent (Variables|Components|GetLeftEquipment) (Variables|Components|GetAvatar) (Variables|Default|GetLeftHandSocket) "SnapToTarget" "KeepRelative" "KeepRelative" true)))))

(fn SetViewCamera
  (bind _chosencam (Variables|Exposed|GetChosenCam))
  (bind _outactors (Actor|GetAllActorsOfClass "/Game/Blueprints/BP_Camera.BP_Camera_C"))
  (bind _output_get (Variables|Default|SetBackupCameras _outactors))
  (Game|Player|SetViewTargetwithBlend (Game|GetPlayerController 0) (select (Utilities|IsValid _chosencam) _chosencam (Utilities|Array|Get(acopy) _output_get)) 0.5 "VTBlend_Linear" 0.0 false))

(fn TransitiontoCamera
  (bind _output_get (Variables|Default|SetNextCamTransition (Utilities|Array|Get(acopy) (Variables|Exposed|GetCameraToTransitionTo) (Variables|Default|GetCurrentCameraIndex))))
  (Game|Player|SetViewTargetwithBlend (Game|GetPlayerController 0) _output_get (Variables|Exposed|GetCameraTransitionSpeed) (Variables|Exposed|GetCameraBlendType) 0.0 false)
  (bind _result (Math|Integer|IncrementInt (Variables|Default|GetCurrentCameraIndex))
    (:%20%20
      (if (== _result (Utilities|Array|Length (Variables|Exposed|GetCameraToTransitionTo)))
        (Utilities|Time|ClearTimerbyFunctionName 0 "TransitionToCamera")))))